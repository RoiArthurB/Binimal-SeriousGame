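; Player controller that runs the front-end menu flow: background, main menu, settings and an error popup.
; A MenuState machine gates startup and settings through Leave_Current_State, which calls Hide_Main when leaving Main Menu.
; Show events lazily create and cache widgets, with main menu and settings switching to UI-only input; both hide events currently set Visible.
; Dismissing an error reloads the Menus level, and End_Game quits by console command.
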(event `Hide_Main`
  (bind _mm_main (`self.MM_Main`))
  ;[1 1 1] hide_main
  (`/Engine/EditorBlueprintResources/StandardMacros.IsValid` _mm_main
    (:`Is Valid`
      (`Widget.SetVisibility` _mm_main "Visible"))))

(event `Start_Over`
  ;[1 1 1] start_over
  (`GameplayStatics.OpenLevel` "Menus"))

(event `End_Game`
  ;[1 1 1] End_Game
  (`KismetSystemLibrary.ExecuteConsoleCommand` "Quit"))

(event `Destroy_Error_Msg`
  (bind _error_msg (`self.Error Msg`))
  ;[1 1 1] Destroy_Error_Msg
  (`/Engine/EditorBlueprintResources/StandardMacros.IsValid` _error_msg
    (:`Is Valid`
      (`Widget.RemoveFromParent` _error_msg)
      (`self.Start_Over`))))

(event `Start_Game`
  ;[1 1 1] Game Startup
  ;;[1 1 1] Start Game
  (`self.Leave_Current_State` "NewEnumerator0"
    (:`New State`
      _)
    (:`Same State`
      _))
  (`self.Show_Background`)
  (`self.Show_MainMenu`))

(event `Show_Background`
  (bind _mm_background (`self.MM_Background`))
  ;[1 1 1] Game Startup
  ;;[1 1 1] Show Background
  (`/Engine/EditorBlueprintResources/StandardMacros.IsValid` _mm_background
    (:`Is Valid`
      (`Widget.SetVisibility` _mm_background "Visible"))
    (:`Is Not Valid`
      (bind _returnvalue (`|CreateWidget` "/Game/GUI/Menus/MM_Background.MM_Background_C" (`GameplayStatics.GetPlayerController` 0)))
      (bind _output_get (set `self.MM_Background` _returnvalue))
      (`UserWidget.AddToViewport` _output_get 0))))

(event `Show_Error_Msg`
  (params (`Error Message` :type Text))
  ;[1 1 1] show_error_msg
  (`/Engine/EditorBlueprintResources/StandardMacros.IsValid` (`self.Error Msg`)
    (:`Is Not Valid`
      (bind _returnvalue (`|CreateWidget` "/Game/GUI/Menus/Error_Msg.Error_Msg_C" self `Error Message`))
      (bind _output_get (set `self.Error Msg` _returnvalue))
      (`UserWidget.AddToViewport` _output_get 0))))

(event `Show_MainMenu`
  (bind _returnvalue (`GameplayStatics.GetPlayerController` 0))
  (bind _mm_main (`self.MM_Main`))
  ;[1 1 1] Game Startup
  ;;[1 1 1] Show Main Menu
  (`/Engine/EditorBlueprintResources/StandardMacros.IsValid` _mm_main
    (:`Is Valid`
      (`Widget.SetVisibility` _mm_main "Visible"))
    (:`Is Not Valid`
      (bind _returnvalue_2 (`|CreateWidget` "/Game/GUI/Menus/MM_Main.MM_Main_C" _returnvalue))
      (bind _output_get (set `self.MM_Main` _returnvalue_2))
      (`UserWidget.AddToViewport` _output_get 0)))
  (`WidgetBlueprintLibrary.SetInputMode_UIOnlyEx` _returnvalue)
  (set `PlayerController.bShowMouseCursor` true _returnvalue))

(event `Show_Settings`
  (bind _mm_settings (`self.MM_Settings`))
  ;[1 1 1] Settings
  ;;[1 1 1] Show Settings
  (`self.Leave_Current_State` "NewEnumerator2"
    (:`New State`
      (`/Engine/EditorBlueprintResources/StandardMacros.IsValid` _mm_settings
        (:`Is Valid`
          (`Widget.SetVisibility` _mm_settings "Visible"))
        (:`Is Not Valid`
          (bind _returnvalue (`|CreateWidget` (`GameplayStatics.GetObjectClass` _mm_settings) self))
          (bind _output_get (set `self.MM_Settings` _returnvalue))
          (`UserWidget.AddToViewport` _output_get 0)))
      (`WidgetBlueprintLibrary.SetInputMode_UIOnlyEx` self))))

(event `Hide_Settings`
  (bind _mm_settings (`self.MM_Settings`))
  ;[1 1 1] Settings
  ;;[1 1 1] Hide Settings
  (`/Engine/EditorBlueprintResources/StandardMacros.IsValid` _mm_settings
    (:`Is Valid`
      (`Widget.SetVisibility` _mm_settings "Visible"))))

(fn `UserConstructionScript`)