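; Answer generator for a binary-to-decimal number level, holding one target number and three decoy decimals.
; BeginPlay rolls the target and decoys through NoDouble, which increments any repeat until it is unique against IntCreated.
; DecimalToBinary builds the target's five-bit string by subtracting powers of two, and BeginPlay prints it on screen.
; Getters expose the target in both forms and each decoy by index.
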(event `self.ReceiveBeginPlay`
  (bind _returnvalue (`KismetMathLibrary.RandomInteger` 31))
  (bind _numberfake (`self.NumberFake`))
  (bind _randomintunique (`self.NoDouble` _returnvalue))
  (bind _output_get (set `self.NumberPlayer` _randomintunique))
  (bind _binaireconv (`self.DecimalToBinary` _output_get))
  (bind _output_get_2 (set `self.NumberPlayerBin` _binaireconv))
  (`KismetSystemLibrary.PrintString` _output_get_2 true true (struct :`R` 0.088547 :`G` 1.0 :`A` 1.0) 10.0)
  (bind _randomintunique_2 (`self.NoDouble` _returnvalue))
  (`KismetArrayLibrary.Array_Insert` _numberfake (`KismetStringLibrary.Conv_IntToString` _randomintunique_2))
  (bind _randomintunique_3 (`self.NoDouble` _returnvalue))
  (`KismetArrayLibrary.Array_Insert` _numberfake (`KismetStringLibrary.Conv_IntToString` _randomintunique_3) 1)
  (bind _randomintunique_4 (`self.NoDouble` _returnvalue))
  (`KismetArrayLibrary.Array_Insert` _numberfake (`KismetStringLibrary.Conv_IntToString` _randomintunique_4) 2))

(fn `GetFakeNumberDecimal`
  (params (index :type Integer :default 0))
  (returns (FakeNumberBin :type String))
  (return (`KismetArrayLibrary.Array_Get` (`self.NumberFake`) index)))

(fn `GetNumberPlayerBin`
  (returns (NumberPlayerBin :type String))
  (return (`self.NumberPlayerBin`)))

(fn `GetNumberPlayerDecimal`
  (returns (NumberPlayerDecimal :type Integer))
  (return (`self.NumberPlayer`)))

(fn `UserConstructionScript`)