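; BoxAnswer is an answer block that shows a number and registers whether it was the correct choice when an actor overlaps it.
; SetTextBin supplies the displayed value and correctness flag, and the text is set shortly after BeginPlay.
; Each tick it rotates along the camera-to-text direction to track the player's view.
; Any overlap destroys it, plays a good or bad sound, and calls the matching FirstPersonHUD feedback.
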(event `self.ReceiveActorBeginOverlap`
  (params (OtherActor :type "Actor Object Reference"))
  ;[1 1 1] Destroy block
  (`ActorComponent.K2_DestroyComponent` (`self.SpriteComponent`))
  (`self.K2_DestroyActor`)
  ;[1 1 1] Test Reponse
  (if (`self.Answer`)
    ;[1 1 1] Feedback ++
    (`KismetSystemLibrary.PrintString` "Good Answer")
    (`GameplayStatics.PlaySound2D` "/Game/Music/AnswersSound/good.good" 10.0)
    (bind _asfirst_person_hud (cast `/Game/FirstPersonBP/Blueprints/FirstPersonHUD` (`PlayerController.GetHUD` (`GameplayStatics.GetPlayerController` 0))))
    (`/Game/FirstPersonBP/Blueprints/FirstPersonHUD.GoodAnswer` _asfirst_person_hud)
    (else
      ;[1 1 1] Feedback --
      (`KismetSystemLibrary.PrintString` "Bad Answer")
      (`GameplayStatics.PlaySound2D` "/Game/Music/AnswersSound/bad.bad" 10.0)
      (bind _asfirst_person_hud_2 (cast `/Game/FirstPersonBP/Blueprints/FirstPersonHUD` (`PlayerController.GetHUD` (`GameplayStatics.GetPlayerController` 0))))
      (`/Game/FirstPersonBP/Blueprints/FirstPersonHUD.WrongAnswerFeedback` _asfirst_person_hud_2))))

(event `self.ReceiveTick`
  (params (DeltaSeconds :type "Float (single-precision)"))
  ;[1 1 1] PlayerLook
  (`self.K2_SetActorRotation` (`KismetMathLibrary.MakeRotFromZ` (- (`SceneComponent.K2_GetComponentLocation` (`self.TextRender`)) (`self.K2_GetActorLocation` (`GameplayStatics.GetPlayerCameraManager` 0))))))

(event `self.ReceiveBeginPlay`
  ;[1 1 1] Init text
  (`KismetSystemLibrary.Delay` 0.2)
  (`TextRenderComponent.K2_SetText` (`self.TextRender`) (`KismetTextLibrary.Conv_StringToText` (`self.NumberPlayerBin`))))

(fn `SetTextBin`
  (params (AnswerLevelBin :type String) (IsGoodAnswer :type Boolean))
  (set `self.NumberPlayerBin` AnswerLevelBin)
  (set `self.Answer` IsGoodAnswer))

(fn `UserConstructionScript`)