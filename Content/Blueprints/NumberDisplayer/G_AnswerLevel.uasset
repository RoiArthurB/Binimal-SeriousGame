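; Level answer holder that picks a random five-bit number on BeginPlay and prints its decimal and binary forms on screen.
; DecimalToBinary builds a zero-padded bit string by successive subtraction of powers of two, from sixteen down to one.
; It also returns those digits parsed as an integer, losing leading zeros.
; Getters expose the decimal value and binary string; RandomInteger(31) never yields 31, so all-ones cannot occur.
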(event `self.ReceiveBeginPlay`
  (bind _output_get (set `self.NumberPlayer` (`KismetMathLibrary.RandomInteger` 31)))
  (`KismetSystemLibrary.PrintString` (`KismetStringLibrary.Conv_IntToString` _output_get) true true (struct :`G` 0.66 :`B` 1.0 :`A` 1.0) 10.0)
  (`self.DecimalToBinary` (`self.NumberPlayer`))
  (`KismetSystemLibrary.PrintString` (`self.binaryString`) true true (struct :`R` 1.0 :`B` 0.6524 :`A` 1.0) 10.0))

(fn `GetNumberPlayerBin`
  (returns (NumberPlayerBin :type String))
  (return (`self.binaryString`)))

(fn `GetNumberPlayerDecimal`
  (returns (NumberPlayerDecimal :type Integer))
  (return (`self.NumberPlayer`)))

(fn `UserConstructionScript`)