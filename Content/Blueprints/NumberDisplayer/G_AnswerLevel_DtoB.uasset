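; Answer generator actor for a decimal-to-binary level, supplying one correct number and three decoys.
; On BeginPlay it draws four random numbers through NoDouble, which increments any repeat until unique, and converts each to a five-bit string with DecimalToBinary.
; Getters expose the answer in decimal and binary plus the binary decoys by index.
; The binary answer is printed on screen as debug output.
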(event `self.ReceiveBeginPlay`
  (bind _returnvalue (`KismetMathLibrary.RandomInteger` 31))
  (bind _numberfake (`self.NumberFake`))
  (bind _randomintunique (`self.NoDouble` _returnvalue))
  (bind _output_get (set `self.NumberPlayer` _randomintunique))
  (bind _binaireconv (`self.DecimalToBinary` _output_get))
  (bind _output_get_2 (set `self.NumberPlayerBin` _binaireconv))
  (`KismetSystemLibrary.PrintString` _output_get_2 true true (struct :`R` 1.0 :`B` 0.6524 :`A` 1.0) 10.0)
  (bind _randomintunique_2 (`self.NoDouble` _returnvalue))
  (bind _binaireconv_2 (`self.DecimalToBinary` _randomintunique_2))
  (`KismetArrayLibrary.Array_Insert` _numberfake _binaireconv_2)
  (bind _randomintunique_3 (`self.NoDouble` _returnvalue))
  (bind _binaireconv_3 (`self.DecimalToBinary` _randomintunique_3))
  (`KismetArrayLibrary.Array_Insert` _numberfake _binaireconv_3 1)
  (bind _randomintunique_4 (`self.NoDouble` _returnvalue))
  (bind _binaireconv_4 (`self.DecimalToBinary` _randomintunique_4))
  (`KismetArrayLibrary.Array_Insert` _numberfake _binaireconv_4 2))

(fn `GetFakeNumberBin`
  (params (index :type Integer :default 0))
  (returns (FakeNumberBin :type String))
  (return (`KismetArrayLibrary.Array_Get` (`self.NumberFake`) index)))

(fn `GetNumberPlayerBin`
  (returns (NumberPlayerBin :type String))
  (return (`self.NumberPlayerBin`)))

(fn `GetNumberPlayerDecimal`
  (returns (NumberPlayerDecimal :type Integer))
  (return (`self.NumberPlayer`)))

(fn `UserConstructionScript`)